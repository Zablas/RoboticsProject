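; BP_Robot is a delivery robot that collects BP_Package actors within a weight limit.
; When its PackageDetector overlaps a package that fits, it adds the weight, stores the destination (package location plus delivery offset) with that weight, and destroys the package.
; It then tells BP_RobotController to start delivering if the robot is full or no packages remain, otherwise to move to another package.
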(event OnComponentBeginOverlap(PackageDetector)
  (params (OverlappedComponent :type Primitive%20Component%20Object%20Reference) (OtherActor :type Actor%20Object%20Reference) (OtherComp :type Primitive%20Component%20Object%20Reference) (OtherBodyIndex :type Integer) (bFromSweep :type Boolean) (SweepResult :type Hit%20Result%20Structure%20%28by%20ref%29))
  (bind _asbp_package (Utilities|Casting|CastToBP_Package OtherActor))
  (if (<= (+ (Variables|Default|GetCurrentWeight) (Variables|/Game/Actors/BP_Package.BP_Package_C|GetWeight _asbp_package)) (Variables|Default|GetMaxWeight))
    (Variables|Default|SetCurrentWeight (+ (Variables|Default|GetCurrentWeight) (Variables|/Game/Actors/BP_Package.BP_Package_C|GetWeight _asbp_package)))
    (Utilities|Array|Add (Variables|Default|GetDeliveryInfoCollection) (Utilities|Struct|MakeStruct_DeliveryInfo (+ (Variables|/Game/Actors/BP_Package.BP_Package_C|GetCoordinatesToDeliverTo _asbp_package) (Transformation|GetActorLocation _asbp_package)) (Variables|/Game/Actors/BP_Package.BP_Package_C|GetWeight _asbp_package)))
    (Actor|DestroyActor _asbp_package)
    (bind _asbp_robot_controller (Utilities|Casting|CastToBP_RobotController (Pawn|GetController)))
    (if (>= (Variables|Default|GetCurrentWeight) (Variables|Default|GetMaxWeight))
      (Default|DeliverPackageEvent _asbp_robot_controller :!label _label)
      (else
        (bind _outactors (Actor|GetAllActorsOfClass "/Game/Actors/BP_Package.BP_Package_C"))
        (if (Utilities|Array|IsEmpty _outactors)
          (goto _label)
          (else
            (Default|MovetoPackage _asbp_robot_controller)))))))

(event EventBeginPlay)

(event Collision|EventActorBeginOverlap
  (params (OtherActor :type Actor%20Object%20Reference)))

(event EventTick
  (params (DeltaSeconds :type Float%20%28single-precision%29)))

(fn ConstructionScript)